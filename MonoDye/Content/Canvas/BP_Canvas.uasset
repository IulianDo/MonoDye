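; BP_Canvas is a drawable canvas actor that paints and erases on the CanvasRT render target at given locations.
; BeginPlay creates pen and eraser dynamic material instances through the mesh's first material slot, then clears the render target to black.
; DrawOnCanvas and EraseFromCanvas pass the 2D location to their material's DrawLocation parameter, then render that material into CanvasRT.
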(event Custom|Erase%20From%20Canvas
  (params (Draw%20Location :type Vector%202D%20Structure))
  ;[1 1 1] Erase
  (Rendering|Material|SetVectorParameterValue (Variables|Default|GetcanvasErasor_MI) "DrawLocation" (Math|Conversions|ToLinearColor(Vector) (Math|Conversions|ToVector(Vector2D) Draw%20Location)) :!class /Script/Engine.MaterialInstanceDynamic)
  (Rendering|DrawMaterialtoRenderTarget (Variables|Default|Getcanvas_RT) (Variables|Default|GetcanvasErasor_MI)))

(event Custom|Draw%20On%20Canvas
  (params (Draw%20Location :type Vector%202D%20Structure))
  ;[1 1 1] Draw
  (Rendering|Material|SetVectorParameterValue (Variables|Default|GetcanvasPen_MI) "DrawLocation" (Math|Conversions|ToLinearColor(Vector) (Math|Conversions|ToVector(Vector2D) Draw%20Location)) :!class /Script/Engine.MaterialInstanceDynamic)
  (Rendering|DrawMaterialtoRenderTarget (Variables|Default|Getcanvas_RT) (Variables|Default|GetcanvasPen_MI)))

(event EventBeginPlay
  (bind _returnvalue (Rendering|Material|CreateDynamicMaterialInstance (Variables|Default|GetStaticMesh) 0 "/Game/Canvas/M_pen.M_pen" "None" :!class /Script/Engine.PrimitiveComponent))
  (Variables|Default|SetcanvasPen_MI _returnvalue)
  (bind _returnvalue_2 (Rendering|Material|CreateDynamicMaterialInstance (Variables|Default|GetStaticMesh) 0 "/Game/Canvas/M_erasor.M_erasor" "None" :!class /Script/Engine.PrimitiveComponent))
  (Variables|Default|SetcanvasErasor_MI _returnvalue_2)
  (Rendering|ClearRenderTarget2D (Variables|Default|Getcanvas_RT)))

(event Collision|EventActorBeginOverlap
  (params (OtherActor :type Actor%20Object%20Reference)))

(event EventTick
  (params (DeltaSeconds :type Float%20%28single-precision%29)))

(fn ConstructionScript)