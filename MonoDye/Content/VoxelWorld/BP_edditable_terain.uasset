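; Editable voxel terrain actor that adds or removes ground at a given UV coordinate.
; On BeginPlay it passes itself to the player's BP_FirstPersonCharacter through SetVoxels.
; CreateTerrain and DestroyTerrain map the UV onto the volume's extent, derived from voxel size and grid size and centered on the actor.
; Each applies three AddSphere or RemoveSphere edits of the same radius, using different fixed Z extents to vary their height.
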(event Custom|Destroy%20Terrain
  (params (UV :type Vector%202D%20Structure))
  (bind _size (Variables|Default|Getsize))
  (bind _size_2 (Variables|Default|Getsize))
  (bind _size_3 (Variables|Default|Getsize))
  (bind _voxelsize (Variables|Default|GetVoxelSize))
  (bind _voxelsize_2 (Variables|Default|GetVoxelSize))
  (bind _voxelsize_3 (Variables|Default|GetVoxelSize))
  (bind _returnvalue (* _voxelsize_2 _size))
  (bind _returnvalue_2 (* _voxelsize_3 _size_3))
  (bind _returnvalue_3 (* _voxelsize _size_2))
  (bind _returnvalue_4 (Math|Vector|MakeVector _returnvalue _returnvalue -2.5e+02))
  (bind _returnvalue_5 (Math|Vector|MakeVector _returnvalue_2 _returnvalue_2 -1e+02))
  (bind _returnvalue_6 (Math|Vector|MakeVector _returnvalue_3 _returnvalue_3 -4e+02))
  (Class|VoxelSphereTools|RemoveSphere 0 (+ (* UV _returnvalue_4) (- (Transformation|GetActorLocation) (/ _returnvalue_4 2))) (Variables|Default|GetRadius))
  (Class|VoxelSphereTools|RemoveSphere 0 (+ (* UV _returnvalue_5) (- (Transformation|GetActorLocation) (/ _returnvalue_5 2))) (Variables|Default|GetRadius))
  (Class|VoxelSphereTools|RemoveSphere 0 (+ (* UV _returnvalue_6) (- (Transformation|GetActorLocation) (/ _returnvalue_6 2))) (Variables|Default|GetRadius)))

(event Custom|Create%20Terrain
  (params (UV :type Vector%202D%20Structure))
  (bind _size (Variables|Default|Getsize))
  (bind _size_2 (Variables|Default|Getsize))
  (bind _size_3 (Variables|Default|Getsize))
  (bind _voxelsize (Variables|Default|GetVoxelSize))
  (bind _voxelsize_2 (Variables|Default|GetVoxelSize))
  (bind _voxelsize_3 (Variables|Default|GetVoxelSize))
  (bind _returnvalue (* _voxelsize _size_3))
  (bind _returnvalue_2 (* _voxelsize_2 _size))
  (bind _returnvalue_3 (* _voxelsize_3 _size_2))
  (bind _returnvalue_4 (Math|Vector|MakeVector _returnvalue _returnvalue -2.5e+02))
  (bind _returnvalue_5 (Math|Vector|MakeVector _returnvalue_2 _returnvalue_2 -1e+02))
  (bind _returnvalue_6 (Math|Vector|MakeVector _returnvalue_3 _returnvalue_3 -4e+02))
  (Class|VoxelSphereTools|AddSphere 0 (+ (* UV _returnvalue_4) (- (Transformation|GetActorLocation) (/ _returnvalue_4 2))) (Variables|Default|GetRadius))
  (Class|VoxelSphereTools|AddSphere 0 (+ (* UV _returnvalue_5) (- (Transformation|GetActorLocation) (/ _returnvalue_5 2))) (Variables|Default|GetRadius))
  (Class|VoxelSphereTools|AddSphere 0 (+ (* UV _returnvalue_6) (- (Transformation|GetActorLocation) (/ _returnvalue_6 2))) (Variables|Default|GetRadius)))

(event EventBeginPlay
  (bind _asbp_first_person_character (Utilities|Casting|CastToBP_FirstPersonCharacter (Game|GetPlayerCharacter 0)))
  (Default|SetVoxels _asbp_first_person_character self))

(fn ConstructionScript)